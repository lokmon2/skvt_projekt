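; Health component that tracks a character's health and also deals its outgoing damage through line-trace hit checks.
; ProcessDamage subtracts from Health and fires the character death signal once IsDead finds it at zero or below.
; TryToHit line-traces between two supplied component locations with debug drawing on, then passes any hit actor to ApplyDamage with BaseDamage.
; The event graph is empty, so all functions rely on outside callers.
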(fn `DealDamageToCharacter`
  (params (DamagedCharacter :type "Actor Object Reference"))
  (`GameplayStatics.ApplyDamage` DamagedCharacter (`self.BaseDamage`)))

(fn `IsDead`
  (returns (IsDead :type Boolean))
  (return (<= (`self.Health`) 0.0)))

(fn `ProcessDamage`
  (params (DamageDealt :type "Float (double-precision)"))
  (set `self.Health` (- (`self.Health`) DamageDealt))
  (if (`self.IsDead`)
    (`self.SignalCharacterDeath`)))

(fn `TryToHit`
  (params (LineTraceStartRef :type "SceneComponent Object Reference") (LineTraceEndRef :type "SceneComponent Object Reference"))
  (bind (_outhit _returnvalue) (`KismetSystemLibrary.LineTraceSingle` :`Start` (`SceneComponent.GetSocketLocation` LineTraceStartRef "None") :`End` (`SceneComponent.GetSocketLocation` LineTraceEndRef "None") :`TraceChannel` "TraceTypeQuery3" :`DrawDebugType` "ForDuration"))
  (if _returnvalue
    (`self.DealDamageToCharacter` (`.HitActor` (`GameplayStatics.BreakHitResult` _outhit)))))