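; Base NPC character that takes damage, attacks and dies through its SkvtHealthComponent.
; Any damage is passed to the component and plays a punch hit-reaction montage.
; The component's death signal turns the mesh into a physics ragdoll, disables movement and destroys the actor after a short timer.
; Attack delegates hit detection to the component, passing line trace start and end references.
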(event `self.SkvtHealthComponent.SignalCharacterDeath`
  (`self.TriggerDeath`))

(event `self.ReceiveAnyDamage`
  (params (Damage :type "Float (single-precision)") (DamageType :type "DamageType Object Reference") (InstigatedBy :type "Controller Object Reference") (DamageCauser :type "Actor Object Reference"))
  (`/Game/Skvt/Systems/Health/AC_HealthComponent.ProcessDamage` (`self.SkvtHealthComponent`) Damage)
  (`self.PlayAnimMontage` "/Game/Skvt/Characters/Animations/Attacks/AM_Hit_punch.AM_Hit_punch"))

(fn `Attack`
  (`/Game/Skvt/Systems/Health/AC_HealthComponent.TryToHit` (`self.SkvtHealthComponent`) (`self.LineTraceStart`) (`self.LineTraceEnd`)))

(fn `FinalizeDeath`
  (`self.K2_DestroyActor`))

(fn `TriggerDeath`
  (`PrimitiveComponent.SetSimulatePhysics` (`self.Mesh`) true)
  (`CharacterMovementComponent.DisableMovement` (`self.CharacterMovement`))
  (`KismetSystemLibrary.K2_SetTimer` null "FinalizeDeath" 5.0))

(fn `UserConstructionScript`)