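; Base NPC character for behavior-tree AI that switches movement speed when it sees or loses the player.
; On possession it caches its AIC_BT_NPCBase controller for later calls.
; PawnSensing sightings raise the walk speed and notify the controller, without checking which pawn was seen.
; A LossPlayer event restores a slower speed and reports the loss to the controller, but nothing in this graph calls it.
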(event `self.ReceivePossessed`
  (params (NewController :type "Controller Object Reference"))
  (bind _asaic_bt_npcbase (cast `/Game/Skvt/Characters/NPC/BehaviorTrees/AIC_BT_NPCBase` (`AIBlueprintHelperLibrary.GetAIController` NewController)))
  (set `self.ControllerRef` _asaic_bt_npcbase))

(event `self.PawnSensing.OnSeePawn`
  (params (Pawn :type "Pawn Object Reference"))
  (set `CharacterMovementComponent.MaxWalkSpeed` 500.0 (`self.CharacterMovement`))
  (`/Game/Skvt/Characters/NPC/BehaviorTrees/AIC_BT_NPCBase.SetSeenPlayer` (`self.ControllerRef`)))

(event `LossPlayer`
  (set `CharacterMovementComponent.MaxWalkSpeed` 250.0 (`self.CharacterMovement`))
  (`/Game/Skvt/Characters/NPC/BehaviorTrees/AIC_BT_NPCBase.SetLossPlayer` (`self.ControllerRef`)))

(fn `UserConstructionScript`
  (`parent.UserConstructionScript`))