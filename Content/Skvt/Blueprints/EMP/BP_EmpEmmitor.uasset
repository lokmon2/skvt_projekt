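; EMP emitter actor that knocks out nearby electric devices when its TriggerEMP event is called.
; TriggerEMP gathers every actor implementing BPI_ElectricDevice and sends DestoryMessage to those within a fixed radius of the static mesh.
; It finds targets by a world-wide interface search and distance check instead of an overlap query, and draws a temporary debug sphere showing the range.
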(event `TriggerEMP`
  (`KismetSystemLibrary.DrawDebugSphere` (`SceneComponent.K2_GetComponentLocation` (`self.StaticMesh`)) 500.0 12 (struct :`R` 1.0 :`A` 1.0) 5.0 1.0)
  (bind _outactors (`GameplayStatics.GetAllActorsWithInterface` "/Game/Skvt/Blueprints/BPI_ElectricDevice.BPI_ElectricDevice_C"))
  (for _array_element _outactors
    (if (<= (`KismetMathLibrary.Vector_Distance` (`self.K2_GetActorLocation` _array_element) (`SceneComponent.K2_GetComponentLocation` (`self.StaticMesh`))) 500.0)
      (message `/Game/Skvt/Blueprints/BPI_ElectricDevice.Destory` _array_element))))

(fn `UserConstructionScript`)