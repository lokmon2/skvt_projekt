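; Interactable button that triggers the EMP emitters in the level matching its value.
; Focus toggles custom depth rendering on the cube, with a stencil value set at BeginPlay, and an interaction widget is exposed through a getter.
; Interaction goes through InteractOnServer to TriggerEMP, which finds all BP_EmpEmmitor actors and fires each whose EMPValue equals the button's ButtonValue.
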(event `self.ReceiveBeginPlay`
  (`PrimitiveComponent.SetCustomDepthStencilValue` (`self.Cube`) 1))

(event `/Game/Skvt/Blueprints/Interaction/BPI_Interaction.Interface_ToggleFocus`
  (params (Focus :type Boolean))
  (`PrimitiveComponent.SetRenderCustomDepth` (`self.Cube`) Focus))

(event `/Game/Skvt/Blueprints/Interaction/BPI_Interaction.InterfaceInteract`
  (`self.InteractOnServer`))

(event `InteractOnServer`
  (`self.TriggerEMP`))

(fn `GetInteractionWidgetRef`
  (returns (Ref :type "WidgetComponent Object Reference"))
  (return (`self.InteractionWidget`)))

(fn `TriggerEMP`
  (bind _outactors (`GameplayStatics.GetAllActorsOfClass` "/Game/Skvt/Blueprints/EMP/BP_EmpEmmitor.BP_EmpEmmitor_C"))
  (for _array_element _outactors
    (if (== (`/Game/Skvt/Blueprints/EMP/BP_EmpEmmitor.EMPValue` _array_element) (`self.ButtonValue`))
      (`/Game/Skvt/Blueprints/EMP/BP_EmpEmmitor.TriggerEMP` _array_element))))

(fn `UserConstructionScript`)