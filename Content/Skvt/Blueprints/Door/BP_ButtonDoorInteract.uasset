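; Interactable button that opens and closes every BP_Door whose DoorValue matches its ButtonValue.
; Interacting calls InteractOnServer, which flips the InteractToggle RepNotify variable; its OnRep searches all BP_Door actors and opens or closes the matches.
; Focus toggles custom depth rendering on the cube for highlighting, and a getter exposes the interaction widget.
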(event `self.ReceiveBeginPlay`
  (`PrimitiveComponent.SetCustomDepthStencilValue` (`self.Cube`) 1))

(event `/Game/Skvt/Blueprints/Interaction/BPI_Interaction.Interface_ToggleFocus`
  (params (Focus :type Boolean))
  (`PrimitiveComponent.SetRenderCustomDepth` (`self.Cube`) Focus))

(event `/Game/Skvt/Blueprints/Interaction/BPI_Interaction.InterfaceInteract`
  (`self.InteractOnServer`))

(event `InteractOnServer`
  (set `self.InteractToggle` (not (`self.InteractToggle`))))

(fn `CloseDoor`
  (bind _outactors (`GameplayStatics.GetAllActorsOfClass` "/Game/Skvt/Blueprints/Door/BP_Door.BP_Door_C"))
  (for _array_element _outactors
    (if (== (`/Game/Skvt/Blueprints/Door/BP_Door.DoorValue` _array_element) (`self.ButtonValue`))
      (`/Game/Skvt/Blueprints/Door/BP_Door.CloseDoor` _array_element))))

(fn `GetInteractionWidgetRef`
  (returns (Ref :type "WidgetComponent Object Reference"))
  (return (`self.InteractionWidget`)))

(fn `OnRep_InteractToggle`
  (if (`self.InteractToggle`)
    (`self.OpenDoor`)
    (else
      (`self.CloseDoor`))))

(fn `OpenDoor`
  (bind _outactors (`GameplayStatics.GetAllActorsOfClass` "/Game/Skvt/Blueprints/Door/BP_Door.BP_Door_C"))
  (for _array_element _outactors
    (if (== (`/Game/Skvt/Blueprints/Door/BP_Door.DoorValue` _array_element) (`self.ButtonValue`))
      (`/Game/Skvt/Blueprints/Door/BP_Door.OpenDoor` _array_element))))

(fn `UserConstructionScript`)