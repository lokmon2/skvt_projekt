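; Interaction component that lets the player focus and use BP_InteractionArea actors by looking at them.
; Each tick it line-traces from the camera and toggles focus as the target changes.
; Interact input fires instantly or, for timed areas, runs a looping timer filling the area's widget progress bar, resetting on release or lost focus.
; Completion calls InteractOnServer, which sends an interface interact message to the area's parent actor.
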(event `self.ReceiveTick`
  (params (DeltaSeconds :type "Float (single-precision)"))
  (`self.Trace`))

(event `TryToInteract`
  (params (In :type Boolean))
  (if In
    (if (`self.IsTracingInteractionArea`)
      (bind _output_get (set `self.Interact Duration` (`/Game/Skvt/Blueprints/Interaction/InteractionArea/BP_InteractionArea.InteractDuration` (`self.FocusedInteractionArea`))))
      (if (> _output_get 0.0)
        (bind _ref (message `/Game/Skvt/Blueprints/Interaction/BPI_Interaction.GetInteractionWidgetRef` (`Actor.GetParentActor` (`self.FocusedInteractionArea`))))
        (bind _aswbp_interaction (cast `/Game/Skvt/UI/Widgets/Interaction/WBP_Interaction` (`WidgetComponent.GetWidget` _ref)))
        (set `self.CurrentInteractionWidgetRef` _aswbp_interaction)
        (bind _returnvalue (`KismetSystemLibrary.K2_SetTimerDelegate` (delegate `UpdateInteractionProgress`) (`self.UpdateInterractionInterval`) true))
        (set `self.InteractionTimer` _returnvalue)
        (else
          (`self.InteractOnServer` (`self.FocusedInteractionArea`)))))
    (else
      (`self.StopInteraction`))))

(event `UpdateInteractionProgress`
  (bind _output_get (set `self.InterractionProgress` (+ (`self.InterractionProgress`) (* (/ 1.0 (`self.Interact Duration`)) (`self.UpdateInterractionInterval`)))))
  (`/Game/Skvt/Materials/ProgressBar/WBP_RoundProgressBar.SetPercent` (`/Game/Skvt/UI/Widgets/Interaction/WBP_Interaction.WBP_RoundProgressBar` (`self.CurrentInteractionWidgetRef`)) _output_get)
  (if (>= (`self.InterractionProgress`) 1.0)
    (`self.StopInteraction`)
    (`self.InteractOnServer` (`self.FocusedInteractionArea`))))

(event `InteractOnServer`
  (params (InteractionArea :type "/Game/Skvt/Blueprints/Interaction/InteractionArea/BP_InteractionArea Object Reference"))
  (message `/Game/Skvt/Blueprints/Interaction/BPI_Interaction.InterfaceInteract` (`Actor.GetParentActor` InteractionArea)))

(fn `StopInteraction`
  (if (> (`self.InterractionProgress`) 0.0)
    (`KismetSystemLibrary.K2_ClearAndInvalidateTimerHandle` (`self.InteractionTimer`))
    (`/Game/Skvt/Materials/ProgressBar/WBP_RoundProgressBar.SetPercent` (`/Game/Skvt/UI/Widgets/Interaction/WBP_Interaction.WBP_RoundProgressBar` (`self.CurrentInteractionWidgetRef`)) 0.0)
    (set `self.InterractionProgress` 0.0)
    (set `self.CurrentInteractionWidgetRef` null)))

(fn `Trace`
  (bind _returnvalue (`GameplayStatics.GetPlayerCameraManager` 0))
  (bind _returnvalue_2 (`Actor.K2_GetActorLocation` _returnvalue))
  (bind (_outhit _returnvalue_3) (`KismetSystemLibrary.LineTraceSingle` _returnvalue_2 (+ _returnvalue_2 (* (`KismetMathLibrary.GetForwardVector` (`Actor.K2_GetActorRotation` _returnvalue)) (`self.Length`))) "TraceTypeQuery1"))
  (if _returnvalue_3
    (bind (_bblockinghit _binitialoverlap _time _distance _location _impactpoint _normal _impactnormal _physmat _hitactor) (`GameplayStatics.BreakHitResult` _outhit))
    (if (!= (`self.FocusedActor`) _hitactor)
      (set `self.FocusedActor` _hitactor)
      (`self.TraceInteractionArea` (== (`GameplayStatics.GetObjectClass` _hitactor) "/Game/Skvt/Blueprints/Interaction/InteractionArea/BP_InteractionArea.BP_InteractionArea_C")))
    (else
      (`self.TraceInteractionArea` false))))

(fn `TraceInteractionArea`
  (params (Trace :type Boolean))
  (if Trace
    (if (`self.IsTracingInteractionArea`)
      (`/Game/Skvt/Blueprints/Interaction/InteractionArea/BP_InteractionArea.ToggleFocus` (`self.FocusedInteractionArea`) false))
    (bind _asbp_interaction_area (cast `/Game/Skvt/Blueprints/Interaction/InteractionArea/BP_InteractionArea` (`self.FocusedActor`)))
    (bind _output_get (set `self.FocusedInteractionArea` _asbp_interaction_area))
    (set `self.IsTracingInteractionArea` true)
    (`/Game/Skvt/Blueprints/Interaction/InteractionArea/BP_InteractionArea.ToggleFocus` _output_get true)
    (elif (`self.IsTracingInteractionArea`)
      (set `self.IsTracingInteractionArea` false)
      (`/Game/Skvt/Blueprints/Interaction/InteractionArea/BP_InteractionArea.ToggleFocus` (`self.FocusedInteractionArea`) false)
      (set `self.FocusedActor` null)
      (set `self.FocusedInteractionArea` null)
      (`self.StopInteraction`))))