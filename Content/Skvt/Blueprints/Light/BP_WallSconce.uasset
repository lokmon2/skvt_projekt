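; Wall sconce light actor that can be toggled on and off or permanently broken into a sparking fixture.
; The construction script applies the configured brightness, color, cone angles and lit state to SconceLight.
; UpdateState flips the light, while the Destory event switches it off for good and fires the Niagara effect.
; Once destroyed, Tick re-activates the Niagara sparks at random intervals of a few seconds.
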(event `self.ReceiveTick`
  (params (DeltaSeconds :type "Float (single-precision)"))
  (if (and (>= (`KismetSystemLibrary.GetGameTimeInSeconds`) (`self.SparksDelay`)) (`self.IsDestroyed`))
    (set `self.SparksDelay` (+ (`KismetSystemLibrary.GetGameTimeInSeconds`) (`KismetMathLibrary.RandomFloatInRange` 1.0 5.0)))
    (`ActorComponent.Activate` (`self.Niagara`) false)))

(event `/Game/Skvt/Blueprints/BPI_ElectricDevice.UpdateState`
  (`self.UpdateLight`))

(event `/Game/Skvt/Blueprints/BPI_ElectricDevice.Destory`
  (`self.Destroy Light`))

(fn `Destroy Light`
  (`ActorComponent.Activate` (`self.Niagara`) false)
  (set `self.SparksDelay` (+ (`KismetSystemLibrary.GetGameTimeInSeconds`) (`KismetMathLibrary.RandomFloatInRange` 1.0 5.0)))
  (set `self.IsDestroyed` true)
  (`self.UpdateLight`))

(fn `Initialize Light`
  (`LightComponent.SetIntensity` (`self.SconceLight`) (`self.Brightness`))
  (`LightComponent.SetLightColor` (`self.SconceLight`) (`self.Color`) true)
  (`SpotLightComponent.SetInnerConeAngle` (`self.SconceLight`) (`self.Inner Cone Angle`))
  (`SpotLightComponent.SetOuterConeAngle` (`self.SconceLight`) (`self.Outer Cone Angle`))
  (`SceneComponent.SetVisibility` (`self.SconceLight`) (`self.IsLit`) false))

(fn `UpdateLight`
  (if (`self.IsDestroyed`)
    (set `self.IsLit` false)
    (else
      (set `self.IsLit` (not (`self.IsLit`)))))
  (`SceneComponent.SetVisibility` (`self.SconceLight`) (`self.IsLit`) false))

(fn `UserConstructionScript`
  (`self.Initialize Light`))