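; BP_SkvtGameMode is a game mode that handles handing player control over to a surviving character.
; It caches the first player controller as BP_SkvtPlayerController on BeginPlay.
; PossesNextCharacter possesses the first BP_SkvtBaseChar that FindNextCharacter finds not dead by scanning all such actors in the world.
; When no living character remains, it tells the controller to create the main menu.
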(event `self.ReceiveBeginPlay`
  (bind _asbp_skvt_player_controller (cast `/Game/Skvt/Characters/BP_SkvtPlayerController` (`GameplayStatics.GetPlayerController` 0)))
  (set `self.ControllserRef` _asbp_skvt_player_controller))

(event `PossesNextCharacter`
  (bind _newpawn (`self.FindNextCharacter`))
  (bind _controllserref (`self.ControllserRef`))
  (`/Engine/EditorBlueprintResources/StandardMacros.IsValid` _newpawn
    (:`Is Valid`
      (`Controller.Possess` _controllserref _newpawn))
    (:`Is Not Valid`
      (`/Game/Skvt/Characters/BP_SkvtPlayerController.CreateMainMenu` _controllserref))))

(fn `FindNextCharacter`
  (returns (NewPawn :type "Pawn Object Reference"))
  (bind _outactors (`GameplayStatics.GetAllActorsOfClass` "/Game/Skvt/Characters/BP_SkvtBaseChar.BP_SkvtBaseChar_C"))
  (for _array_element _outactors
    (if (not (`/Game/Skvt/Characters/BP_SkvtBaseChar.IsDead` _array_element))
      (return _array_element))))

(fn `UserConstructionScript`)